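; BP_WoodChopGameBase is a wood-chop game base Blueprint that starts the music on a Quartz clock.
; On BeginPlay it creates a 4/4 "MainClock", sets its tempo and queues the 2D music to play quantized to the beat.
; The clock starts only when the quantization callback reports the play command as queued, so music and clock begin in step.
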(event `self.ReceiveBeginPlay`
  (`parent.ReceiveBeginPlay`)
  (bind _returnvalue (`QuartzSubsystem.CreateNewClock` (subsystem `QuartzSubsystem`) "MainClock" (make `QuartzClockSettings` (make `QuartzTimeSignature` 4)) false true))
  (bind _clockhandle (`QuartzClockHandle.SetBeatsPerMinute` :`self` _returnvalue :`QuantizationBoundary` (make `QuartzQuantizationBoundary` "Beat" 1.0 "TransportRelative") :`BeatsPerMinute` 100.0))
  (set `self.MainClock` _clockhandle)
  (bind _returnvalue_2 (`GameplayStatics.SpawnSound2D` (`self.Music`) 1.0 1.0 0.0 null))
  (`AudioComponent.PlayQuantized` _returnvalue_2 (`self.MainClock`) (make `QuartzQuantizationBoundary` "Beat" 1.0 "TransportRelative") (delegate `CustomEvent_0`) 0.0 0.0 1.0 "Linear"))

(event `CustomEvent_0`
  (params (EventType :type "EQuartzCommandDelegateSubType Enum" :default "CommandOnFailedToQueue") (Name :type Name))
  (switch `EQuartzCommandDelegateSubType` "CommandOnFailedToQueue"
    (:`CommandOnQueued`
      (`QuartzClockHandle.StartClock` (`self.MainClock`)))))

(fn `UserConstructionScript`
  (`parent.UserConstructionScript`))