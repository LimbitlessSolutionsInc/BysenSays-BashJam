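; Player for a rhythm wood-chopping minigame, scoring flex or Space inputs on timing against the gamemode's beats.
; Inputs share a cooldown-gated DoOnce that plays an axe montage and compares hit time to the nearer beat.
; On chop beats, a linear offset-to-points formula feeds the team point counter and a tiered success-message widget.
; Missed-beat calls decrement lives; at zero, input is disabled and a timeline spins, shrinks and hides the player.
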(event `self.ReceiveBeginPlay`
  (bind _asbp_wood_chop_gamemode (cast `/Game/Blueprints/BP_WoodChopGamemode` (`GameplayStatics.GetGameMode`)))
  (set `self.Gamemode` _asbp_wood_chop_gamemode))

(event `EnhancedInput|/LimbitlessBluetoothPlugin/InputActions/IA_LightFlex`
  (params (ActionValue :type Boolean) (ElapsedSeconds :type "Float (double-precision)") (TriggeredSeconds :type "Float (double-precision)") (InputAction :type "InputAction Object Reference" :default "/LimbitlessBluetoothPlugin/InputActions/IA_LightFlex.IA_LightFlex"))
  (bind _playernumber (`self.PlayerNumber`))
  (bind _gamemode (`self.Gamemode`))
  (bind _basepointcounter (`/Game/Blueprints/BP_WoodChopGamemode.BasePointCounter` (`self.Gamemode`)))
  (:`Triggered`
    (`|DoOnceMultiInput` :!label _label
      (:`A Out`
        (set `self.CooldownTime` (`self.CooldownReset`))
        (`|PlayMontage` (`self.BP_PlayerMeshComponent`) "/Game/Gnome/AM_ModChara_AxeHit.AM_ModChara_AxeHit"
          (:`then`
            (bind _output_get (set `self.PlayerFlexTime` (`GameplayStatics.GetTimeSeconds`)))
            (bind _returnvalue (`KismetMathLibrary.Abs` (- _output_get (`/Game/Blueprints/BP_WoodChopGamemode.TimeAtLastBeat` _gamemode))))
            (bind _returnvalue_2 (`KismetMathLibrary.Abs` (- _output_get (`/Game/Blueprints/BP_WoodChopGamemode.TimeAtNextBeat` _gamemode))))
            (`/Engine/EditorBlueprintResources/StandardMacros.CompareFloat` _returnvalue _returnvalue_2
              (:`>`
                (bind _output_get_2 (set `self.PlayerHitOffset` _returnvalue_2 :!label _label_2)) ; Use next beat
                (if (`/Game/Blueprints/BP_WoodChopGamemode.NextBeatHasChop` (`self.Gamemode`))
                  (`KismetSystemLibrary.PrintString` (`KismetStringLibrary.Conv_DoubleToString` _returnvalue_2))
                  (bind _points (`self.AwardPointsForChop` _output_get_2))
                  (`self.DisplaySuccessText` _points)
                  (`BasePointCounter.AddPoints` _basepointcounter _playernumber _points)
                  (`KismetSystemLibrary.PrintString` (`KismetStringLibrary.Conv_IntToString` _points) :!label _label_3)))
              (:`==`
                (goto _label_2))
              (:`<`
                (bind _output_get_3 (set `self.PlayerHitOffset` _returnvalue)) ; Use previous beat
                (if (`/Game/Blueprints/BP_WoodChopGamemode.LastBeatHadChop` (`self.Gamemode`))
                  (`KismetSystemLibrary.PrintString` "hit late for last beat")
                  (bind _points_2 (`self.AwardPointsForChop` _output_get_3))
                  (`self.DisplaySuccessText` _points_2)
                  (`BasePointCounter.AddPoints` _basepointcounter _playernumber _points_2)
                  (goto _label_3))))))))))

(event `self.ReceiveTick`
  (params (DeltaSeconds :type "Float (single-precision)"))
  (bind _cooldowntime (`self.CooldownTime`))
  ;[1 1 1] Decrement Cooldown Timer
  (`/Engine/EditorBlueprintResources/StandardMacros.CompareFloat` _cooldowntime
    (:`>`
      (set `self.CooldownTime` (- _cooldowntime DeltaSeconds)))
    (:`==`
      (goto _label :!via `Reset In`))
    (:`<`
      (goto _label :!via `Reset In`))))

(event `EnhancedInput|/LimbitlessBluetoothPlugin/InputActions/IA_MediumFlex`
  (params (ActionValue :type Boolean) (ElapsedSeconds :type "Float (double-precision)") (TriggeredSeconds :type "Float (double-precision)") (InputAction :type "InputAction Object Reference" :default "/LimbitlessBluetoothPlugin/InputActions/IA_MediumFlex.IA_MediumFlex"))
  (:`Triggered`
    (goto _label)))

(event `EnhancedInput|/LimbitlessBluetoothPlugin/InputActions/IA_StrongFlex`
  (params (ActionValue :type Boolean) (ElapsedSeconds :type "Float (double-precision)") (TriggeredSeconds :type "Float (double-precision)") (InputAction :type "InputAction Object Reference" :default "/LimbitlessBluetoothPlugin/InputActions/IA_StrongFlex.IA_StrongFlex"))
  (:`Triggered`
    (goto _label)))

(event `Key|SpaceBar`
  (params (Key :type "Key Structure"))
  (:`Pressed`
    (goto _label)))

(event `player missed beat`
  ;[1 1 1] Call this when player misses a beat
  (bind _result (`/Engine/EditorBlueprintResources/StandardMacros.DecrementInt` (`self.PlayerLives`))
    (:`  `
      (if (<= _result 0)
        (`self.Remove (Hide) Player`)))))

(event `Remove (Hide) Player`
  ;[1 1 1] Remove Player from Game          (Player Eliminated)
  (`self.DisableInput` null)
  (bind (_direction _rotation_speed_curve _shrink_curve) (`Timeline|death timeline`)
    (:`Update`
      ;;[1 1 1] Rotate Animation
      (`self.K2_AddActorLocalRotation` (`KismetMathLibrary.MakeRotator` 0.0 0.0 (* _rotation_speed_curve (`GameplayStatics.GetWorldDeltaSeconds`))))
      ;;[1 1 1] Shrink Animation
      (`self.SetActorScale3D` (`KismetMathLibrary.MakeVector` _shrink_curve _shrink_curve _shrink_curve)))
    (:`Finished`
      ;;[1 1 1] toggle visibility      (set to invisible)
      (`SceneComponent.SetVisibility` (`self.BP_PlayerMeshComponent`) false false))))

(fn `AwardPointsForChop`
  (params (HitOffset :type "Float (double-precision)"))
  (returns (Points :type Integer))
  (return (`KismetMathLibrary.Abs_Int` (`KismetMathLibrary.Round` (`KismetMathLibrary.Lerp` 0.0 10.0 (- 1.0 (/ HitOffset 0.3)))))))

(fn `DisplaySuccessText`
  (params (PointNum :type Integer))
  (bind _returnvalue (`WidgetComponent.GetWidget` (`self.SuccessMessage`)))
  (switch `int` PointNum
    (:`Default`
      (bind _output_get (set `self.CurrSuccessText` "OKAY!" :!label _label))
      (bind _output_get_2 (set `self.CurrSuccessColor` (struct :`R` 0.661458 :`G` 0.065111 :`A` 1.0)))
      (bind _asbp_success_message (cast `/Game/Blueprints/BP_SuccessMessage` _returnvalue))
      (`/Game/Blueprints/BP_SuccessMessage.SetWordText` _asbp_success_message _output_get _output_get_2))
    (:`0`
      (goto _label))
    (:`1`
      (goto _label))
    (:`2`
      (goto _label))
    (:`3`
      (goto _label))
    (:`4`
      (goto _label))
    (:`5`
      (bind _output_get_3 (set `self.CurrSuccessText` "GOOD!" :!label _label_2))
      (bind _output_get_4 (set `self.CurrSuccessColor` (struct :`R` 0.562653 :`G` 0.661458 :`A` 1.0)))
      (bind _asbp_success_message_2 (cast `/Game/Blueprints/BP_SuccessMessage` _returnvalue))
      (`/Game/Blueprints/BP_SuccessMessage.SetWordText` _asbp_success_message_2 _output_get_3 _output_get_4))
    (:`6`
      (goto _label_2))
    (:`7`
      (bind _output_get_5 (set `self.CurrSuccessText` "AWESOME!" :!label _label_3))
      (bind _output_get_6 (set `self.CurrSuccessColor` (struct :`R` 0.040746 :`G` 0.661458 :`A` 1.0)))
      (bind _asbp_success_message_3 (cast `/Game/Blueprints/BP_SuccessMessage` _returnvalue))
      (`/Game/Blueprints/BP_SuccessMessage.SetWordText` _asbp_success_message_3 _output_get_5 _output_get_6))
    (:`8`
      (goto _label_3))
    (:`9`
      (bind _output_get_7 (set `self.CurrSuccessText` "PERFECT!" :!label _label_4))
      (bind _output_get_8 (set `self.CurrSuccessColor` (struct :`R` 0.237449 :`B` 0.661458 :`A` 1.0)))
      (bind _asbp_success_message_4 (cast `/Game/Blueprints/BP_SuccessMessage` _returnvalue))
      (`/Game/Blueprints/BP_SuccessMessage.SetWordText` _asbp_success_message_4 _output_get_7 _output_get_8))
    (:`10`
      (goto _label_4))))

(fn `UserConstructionScript`)