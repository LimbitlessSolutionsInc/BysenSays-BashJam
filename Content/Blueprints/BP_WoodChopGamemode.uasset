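; Game mode for a wood-chopping rhythm game, running music on a Quartz clock at a fixed tempo.
; BeginPlay and a game-reset handler share setup that creates the clock and queues quantized music playback.
; Once queued, the clock starts and a beat subscription records each beat's time.
; Player chop hits call a beat-match check that is still an empty stub, with next-beat time merely copying the last.
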(event `OnGameReset_Event`
  (add `MinigameBase.OnGameReset` (delegate `CustomEvent_1`)))

(event `CustomEvent_1`
  (`parent.ReceiveBeginPlay` :!label _label)
  (bind _returnvalue (`QuartzSubsystem.CreateNewClock` (subsystem `QuartzSubsystem`) "MainClock" (make `QuartzClockSettings` (make `QuartzTimeSignature` 4)) false true))
  (bind _clockhandle (`QuartzClockHandle.SetBeatsPerMinute` :`self` _returnvalue :`QuantizationBoundary` (make `QuartzQuantizationBoundary` "Beat" 1.0 "TransportRelative") :`BeatsPerMinute` 100.0))
  (set `self.MainClock` _clockhandle)
  (bind _returnvalue_2 (`GameplayStatics.SpawnSound2D` (`self.Music`) 1.0 1.0 0.0 null))
  (`AudioComponent.PlayQuantized` _returnvalue_2 (`self.MainClock`) (make `QuartzQuantizationBoundary` "Beat" 1.0 "TransportRelative") (delegate `CustomEvent_0`) 0.0 0.0 1.0 "Linear"))

(event `self.ReceiveBeginPlay`
  (goto _label))

(event `CustomEvent_0`
  (params (EventType :type "EQuartzCommandDelegateSubType Enum" :default "CommandOnFailedToQueue") (Name :type Name))
  (switch `EQuartzCommandDelegateSubType` EventType
    (:`CommandOnQueued`
      (bind _clockhandle (`QuartzClockHandle.StartClock` (`self.MainClock`)))
      (`QuartzClockHandle.SubscribeToQuantizationEvent` _clockhandle "Beat" (delegate `CustomEvent`)))))

(event `CustomEvent`
  (params (ClockName :type Name) (QuantizationType :type "EQuartzCommandQuantization Enum" :default "Bar") (NumBars :type Integer) (Beat :type Integer) (BeatFraction :type "Float (single-precision)"))
  (set `self.TimeAtLastBeat` (`GameplayStatics.GetTimeSeconds`))
  (set `self.TimeAtNextBeat` (`self.TimeAtLastBeat`)))

(event `Player Hit Chop (Flexed)`
  (params (Target :type "Self Object Reference"))
  (cast `/Game/Blueprints/BP_WoodChopGamePlayer` Target)
  (`self.Check if Beat Matches Chop`))

(event `Check if Beat Matches Chop`
  (if true
    _))

(fn `UserConstructionScript`
  (`parent.UserConstructionScript`))