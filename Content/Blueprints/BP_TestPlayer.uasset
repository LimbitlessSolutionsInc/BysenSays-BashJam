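; Test player for a wood-chop rhythm game that times flex inputs against the gamemode's beat.
; Light, medium and strong flex actions and Space share one do-once gate, which starts a cooldown.
; It prints "Chop!" when the absolute difference between game time and time since last beat meets or exceeds the lenience.
; Tick counts the cooldown down and resets the gate only when it exactly equals zero.
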(event `self.ReceiveBeginPlay`
  (bind _asbp_wood_chop_gamemode (cast `/Game/Blueprints/BP_WoodChopGamemode` (`GameplayStatics.GetGameMode`)))
  (set `self.Gamemode` _asbp_wood_chop_gamemode))

(event `EnhancedInput|/LimbitlessBluetoothPlugin/InputActions/IA_LightFlex`
  (params (ActionValue :type Boolean) (ElapsedSeconds :type "Float (double-precision)") (TriggeredSeconds :type "Float (double-precision)") (InputAction :type "InputAction Object Reference" :default "/LimbitlessBluetoothPlugin/InputActions/IA_LightFlex.IA_LightFlex"))
  (:`Triggered`
    (`|DoOnceMultiInput` :!label _label
      (:`A Out`
        (set `self.CooldownTime` (`self.CooldownReset`))
        (bind _output_get (set `self.PlayerFlexTime` (`GameplayStatics.GetTimeSeconds`)))
        (bind _timesincelastbeat (`/Game/Blueprints/BP_WoodChopGamemode.GetTimeSinceLastBeat` (`self.Gamemode`)))
        (bind _output_get_2 (set `self.PlayerHitOffset` (`KismetMathLibrary.Abs` (- _output_get _timesincelastbeat))))
        (`/Engine/EditorBlueprintResources/StandardMacros.CompareFloat` _output_get_2 (`self.PlayerHitLenience`)
          (:`>`
            _)
          (:`==`
            _))
        (`KismetSystemLibrary.PrintString` "Chop!")))))

(event `self.ReceiveTick`
  (params (DeltaSeconds :type "Float (single-precision)"))
  (bind _cooldowntime (`self.CooldownTime`))
  ;[1 1 1] Decrement Cooldown Timer
  (`/Engine/EditorBlueprintResources/StandardMacros.CompareFloat` _cooldowntime
    (:`>`
      (set `self.CooldownTime` (- _cooldowntime DeltaSeconds)))
    (:`==`
      (goto _label :!via `Reset In`))))

(event `EnhancedInput|/LimbitlessBluetoothPlugin/InputActions/IA_MediumFlex`
  (params (ActionValue :type Boolean) (ElapsedSeconds :type "Float (double-precision)") (TriggeredSeconds :type "Float (double-precision)") (InputAction :type "InputAction Object Reference" :default "/LimbitlessBluetoothPlugin/InputActions/IA_MediumFlex.IA_MediumFlex"))
  (:`Triggered`
    (goto _label)))

(event `EnhancedInput|/LimbitlessBluetoothPlugin/InputActions/IA_StrongFlex`
  (params (ActionValue :type Boolean) (ElapsedSeconds :type "Float (double-precision)") (TriggeredSeconds :type "Float (double-precision)") (InputAction :type "InputAction Object Reference" :default "/LimbitlessBluetoothPlugin/InputActions/IA_StrongFlex.IA_StrongFlex"))
  (:`Triggered`
    (goto _label)))

(event `Key|SpaceBar`
  (params (Key :type "Key Structure"))
  (:`Pressed`
    (goto _label)))

(fn `UserConstructionScript`)